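; BP_MagicMissile is a magic missile spell projectile that plays a cast sound on spawn.
; When its sphere overlaps a component not tagged Player, it calls ApplyHit on the target.
; It then deactivates the trail, hides the sphere, disables collision and spawns an explosion effect.
; The actor destroys itself after a short delay.
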(event `self.ReceiveBeginPlay`
  (`GameplayStatics.PlaySoundAtLocation` "/Game/Sounds/MagicSpell_Cue.MagicSpell_Cue" (`self.K2_GetActorLocation`) (struct) 1.0 1.0 0.0 null null null null))

(event `self.Sphere.OnComponentBeginOverlap`
  (params (OverlappedComponent :type "PrimitiveComponent Object Reference") (OtherActor :type "Actor Object Reference") (OtherComp :type "PrimitiveComponent Object Reference") (OtherBodyIndex :type Integer) (bFromSweep :type Boolean) (SweepResult :type "HitResult Structure (by ref)"))
  (if (not (`ActorComponent.ComponentHasTag` OtherComp "Player"))
    (`self.ApplyHit` OtherActor OtherComp)
    (`ActorComponent.Deactivate` (`self.MissileTrailVFX`))
    (`SceneComponent.SetHiddenInGame` (`self.Sphere`) true false)
    (`self.SetActorEnableCollision` false)
    (`NiagaraFunctionLibrary.SpawnSystemAtLocation` "/Game/Andrew_Content/MissileExplode.MissileExplode" (`SceneComponent.K2_GetComponentLocation` (`self.Sphere`)))
    (`KismetSystemLibrary.Delay` 2.2)
    (`self.K2_DestroyActor`)))

(fn `UserConstructionScript`)