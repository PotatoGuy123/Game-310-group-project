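; BP_FireBall is a fireball spell actor that explodes on overlap.
; Sphere overlaps, except with ExplosionCheck or Player-tagged components, fire a radial impulse and spawn the explosion effect.
; Short delays then deactivate the trail and destroy the actor; its SetActorHiddenInGame call passes false, so nothing is hidden.
; The loop over characters in ExplosionCheck is empty, and ApplyHit is disconnected, so this graph applies no hits.
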(event `self.ReceiveBeginPlay`
  (`parent.ReceiveBeginPlay`))

(event `self.ReceiveActorBeginOverlap`
  (params (OtherActor :type "Actor Object Reference"))
  (`parent.ReceiveActorBeginOverlap` OtherActor))

(event `self.Sphere.OnComponentBeginOverlap`
  (params (OverlappedComponent :type "PrimitiveComponent Object Reference") (OtherActor :type "Actor Object Reference") (OtherComp :type "PrimitiveComponent Object Reference") (OtherBodyIndex :type Integer) (bFromSweep :type Boolean) (SweepResult :type "HitResult Structure (by ref)"))
  (if (and (!= OtherComp (`self.ExplosionCheck`)) (not (`ActorComponent.ComponentHasTag` OtherComp "Player")))
    (`RadialForceComponent.FireImpulse` (`self.RadialForce`))
    (for (_array_element _array_index) (`PrimitiveComponent.GetOverlappingActors` (`self.ExplosionCheck`) "/Script/Engine.Character")
      _)
    (`NiagaraFunctionLibrary.SpawnSystemAtLocation` "/Game/Andrew_Content/FireballExplode.FireballExplode" (`SceneComponent.K2_GetComponentLocation` (`self.Sphere`)))
    (`KismetSystemLibrary.Delay` 0.1)
    (`ActorComponent.Deactivate` (`self.FireballTrailVFX`))
    (`self.SetActorHiddenInGame` false)
    (`KismetSystemLibrary.Delay` 2.2)
    (`self.K2_DestroyActor`)))

(fn `UserConstructionScript`
  (`parent.UserConstructionScript`))