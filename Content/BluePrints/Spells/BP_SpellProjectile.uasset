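; Spell projectile actor that plays a magic cast sound at its location on spawn and damages what it hits.
; Sphere overlaps feed ApplyHit, which ignores components tagged Player, otherwise sends TakeDamageMessage with DamageAmount to the other actor and destroys the projectile.
; ApplyHitEffect is an empty function that nothing in this graph calls.
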(event `self.ReceiveBeginPlay`
  (`GameplayStatics.PlaySoundAtLocation` "/Game/Sounds/MagicSpell_Cue.MagicSpell_Cue" (`self.K2_GetActorLocation`) (struct) 1.0 1.0 0.0 null null null null))

(event `self.Sphere.OnComponentBeginOverlap`
  (params (OverlappedComponent :type "PrimitiveComponent Object Reference") (OtherActor :type "Actor Object Reference") (OtherComp :type "PrimitiveComponent Object Reference") (OtherBodyIndex :type Integer) (bFromSweep :type Boolean) (SweepResult :type "HitResult Structure (by ref)"))
  (`self.ApplyHit` OtherActor OtherComp))

(fn `ApplyHit`
  (params (`Other Actor` :type "Object Object Reference") (`Other Comp` :type "ActorComponent Object Reference"))
  (if (not (`ActorComponent.ComponentHasTag` `Other Comp` "Player"))
    (message `/Game/BluePrints/Component/BPI_HealthInterface.TakeDamage` `Other Actor` (`self.Damage Amount`))
    (`self.K2_DestroyActor`)))

(fn `ApplyHitEffect`)

(fn `UserConstructionScript`)