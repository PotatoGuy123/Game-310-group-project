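; Health component that tracks an actor's current health against a maximum, starting at full on BeginPlay.
; TakeDamage subtracts from health and fires the Die dispatcher once it drops to zero or below, with no guard against repeated calls.
; HealDamage adds health and clamps it to the maximum.
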(event `self.ReceiveBeginPlay`
  (set `self.CurrentHealth` (`self.MaxHealth`)))

(fn `HealDamage`
  (params (HealAmount :type "Float (double-precision)"))
  (bind _output_get (set `self.CurrentHealth` (+ (`self.CurrentHealth`) HealAmount)))
  (if (> _output_get (`self.MaxHealth`))
    (set `self.CurrentHealth` (`self.MaxHealth`))))

(fn `TakeDamage`
  (params (DamageAmount :type "Float (double-precision)"))
  (bind _output_get (set `self.CurrentHealth` (- (`self.CurrentHealth`) DamageAmount)))
  (if (<= _output_get 0.0)
    (`self.Die`)))