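; Mana component that tracks an actor's current mana and passively regenerates it over time.
; On BeginPlay it fills mana to the maximum and starts a looping timer that periodically adds the regen rate through IncreaseCurrentMana.
; Increases clamp at the maximum, while decreases have no lower bound.
; Both change functions call CallRecalibrateManaBar after updating the value.
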(event `self.ReceiveBeginPlay`
  (set `self.CurrentMana` (`self.MaxMana`))
  (`KismetSystemLibrary.K2_SetTimerDelegate` (delegate `Regenerate Mana`) 0.5 true))

(event `Regenerate Mana`
  (`self.IncreaseCurrentMana` (`self.ManaRegenRate`)))

(fn `DecreaseCurrentMana`
  (params (DamageAmount :type "Float (double-precision)"))
  (set `self.CurrentMana` (- (`self.CurrentMana`) DamageAmount))
  (`self.RecalibrateManaBar`))

(fn `IncreaseCurrentMana`
  (params (HealAmount :type "Float (double-precision)"))
  (bind _output_get (set `self.CurrentMana` (+ (`self.CurrentMana`) HealAmount)))
  (if (> _output_get (`self.MaxMana`))
    (set `self.CurrentMana` (`self.MaxMana`)))
  (`self.RecalibrateManaBar`))