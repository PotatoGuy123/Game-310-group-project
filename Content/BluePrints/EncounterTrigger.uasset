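; EncounterTrigger is a box trigger that starts a combat encounter with its RelatedEnemies and rewards the player for clearing it.
; The first overlap of any kind disables the box; if the component is tagged Player, each enemy's AI switches to attacking and the Wall is unhidden with a sound.
; Bound health-component death events count down EnemiesLeft; at zero, the Wall is destroyed, an end sound plays and the player is healed.
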(event `self.Box.OnComponentBeginOverlap`
  (params (OverlappedComponent :type "PrimitiveComponent Object Reference") (OtherActor :type "Actor Object Reference") (OtherComp :type "PrimitiveComponent Object Reference") (OtherBodyIndex :type Integer) (bFromSweep :type Boolean) (SweepResult :type "HitResult Structure (by ref)"))
  (`PrimitiveComponent.SetCollisionEnabled` (`self.Box`) "NoCollision")
  (if (`ActorComponent.ComponentHasTag` OtherComp "Player")
    (`KismetSystemLibrary.PrintString` "BEGIN")
    (for _array_element (`self.RelatedEnemies`)
      (bind _asaic_enemy_base (cast `/Game/Enemies/AI/AIC_EnemyBase` (`AIBlueprintHelperLibrary.GetAIController` _array_element)))
      (`/Game/Enemies/AI/AIC_EnemyBase.SetStateAsAttacking` _asaic_enemy_base)
      (set `self.Enemies Left` (+ (`self.Enemies Left`) 1))
      (add `/Game/BluePrints/Component/HealthComponent.Die` (`/Game/Enemies/BP_EnemyBase.HealthComponent` _array_element) (delegate `EnemyDied`))
      (`self.SetActorHiddenInGame` (`self.Wall`) false)
      (`GameplayStatics.PlaySoundAtLocation` "/Game/Sounds/BeginCombatSound.BeginCombatSound" (`self.K2_GetActorLocation`) (struct) 1.0 1.0 0.0 null null null null))))

(event `EnemyDied`
  (bind _output_get (set `self.Enemies Left` (- (`self.Enemies Left`) 1)))
  (if (<= _output_get 0)
    (`self.K2_DestroyActor` (`self.Wall`))
    (`GameplayStatics.PlaySoundAtLocation` "/Game/Sounds/EndCombatSound_Cue.EndCombatSound_Cue" (`self.K2_GetActorLocation`) (struct) 1.0 1.0 0.0 null null null null)
    (message `/Game/BluePrints/Component/BPI_HealthInterface.HealDamage` (`GameplayStatics.GetPlayerCharacter` 0) 50.0)))

(fn `UserConstructionScript`)