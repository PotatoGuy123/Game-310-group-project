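; BP_ElectroHandsUnlock is a pickup, shown as a wine bottle with a light and VFX, that unlocks the player's ElectroHands ability.
; When BP_ThirdPersonCharacter overlaps its sphere, it calls UnlockElectroHands and fires the "Heal" trigger on that character's Soundtrack.
; It then hides the bottle and light, deactivates the VFX and disables collision, destroying itself after a short delay.
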(event `self.Sphere.OnComponentBeginOverlap`
  (params (OverlappedComponent :type "PrimitiveComponent Object Reference") (OtherActor :type "Actor Object Reference") (OtherComp :type "PrimitiveComponent Object Reference") (OtherBodyIndex :type Integer) (bFromSweep :type Boolean) (SweepResult :type "HitResult Structure (by ref)"))
  (bind _asbp_third_person_character (cast `/Game/ThirdPerson/Blueprints/BP_ThirdPersonCharacter` OtherActor))
  (`/Game/ThirdPerson/Blueprints/BP_ThirdPersonCharacter.Unlock Electro hands` _asbp_third_person_character)
  (`AudioParameterControllerInterface.SetTriggerParameter` (`/Game/ThirdPerson/Blueprints/BP_ThirdPersonCharacter.Soundtrack` _asbp_third_person_character) "Heal")
  (`SceneComponent.SetHiddenInGame` (`self.WineBottle`) true false)
  (`SceneComponent.SetHiddenInGame` (`self.PointLight`) true false)
  (`ActorComponent.Deactivate` (`self.PickupVFX`))
  (`self.SetActorEnableCollision` false)
  (`KismetSystemLibrary.Delay` 2.1)
  (`self.K2_DestroyActor`))

(fn `UserConstructionScript`)