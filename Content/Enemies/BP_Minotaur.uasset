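; BP_Minotaur is an AI-driven enemy character that knocks characters back and drops an alcohol pickup on death.
; SetMoveSpeed switches max walk speed between walk, run and charge, while Hit Effect launches the struck character along the look-at direction from the Minotaur.
; DieEffect calls OnDeath, spawns the pickup, disables collision and gravity, stops AI logic, then plays the death montage and destroys the actor after a short delay.
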(event `self.ReceiveBeginPlay`
  (`parent.ReceiveBeginPlay`))

(event `DeathAnim`
  (`|PlayMontage` (`self.Mesh`) "/Game/Enemies/Models/Minotaur/MinotaurDeath_Montage.MinotaurDeath_Montage"
    (:`then`
      (`KismetSystemLibrary.Delay` 3.0)
      (`self.K2_DestroyActor`))))

(fn `DieEffect`
  (`self.OnDeath`)
  (`|SpawnActorFromClass` "/Game/BluePrints/BP_AlchoholPickup.BP_AlchoholPickup_C" (`self.GetTransform`) "Undefined" "MultiplyWithRoot" null null)
  (`self.SetActorEnableCollision` false)
  (`self.SetActorHiddenInGame` false)
  (set `CharacterMovementComponent.GravityScale` 0.0 (`self.CharacterMovement`))
  (`BrainComponent.StopLogic` (`AIController.BrainComponent` (`AIBlueprintHelperLibrary.GetAIController` self)) "")
  (`self.DeathAnim`))

(fn `Hit Effect`
  (params (`Other Actor` :type "Actor Object Reference"))
  (bind _ascharacter (cast `Character` `Other Actor`))
  (`self.LaunchCharacter` _ascharacter (* (`KismetMathLibrary.GetForwardVector` (`KismetMathLibrary.FindLookAtRotation` (`self.K2_GetActorLocation`) (`self.K2_GetActorLocation` `Other Actor`))) (`self.Attack knockback`)) true false))

(fn `NewFunction_0`)

(fn `SetMoveSpeed`
  (params (`New move speed` :type "/Game/Enemies/AI/Enmus/MoveSpeeds Enum" :default "NewEnumerator0"))
  (set `CharacterMovementComponent.MaxWalkSpeed` (select `/Game/Enemies/AI/Enmus/MoveSpeeds` `New move speed` :`NewEnumerator0` (`self.WalkSpeed`) :`NewEnumerator1` (`self.RunSpeed`) :`NewEnumerator2` (`self.ChargeSpeed`) :!type "Float (single-precision)") (`self.CharacterMovement`)))

(fn `UserConstructionScript`
  (`parent.UserConstructionScript`))