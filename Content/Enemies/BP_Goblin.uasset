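; Goblin enemy Blueprint that adds goblin-specific feedback on top of a parent enemy class.
; Overrides of the aggro, attack sound, hurt and death functions each call the parent, then fire a matching named trigger parameter on the Goblin component, which appears to be MetaSound-style audio.
; The event graph and construction script add no logic of their own.
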(fn `AggroUnits`
  (`parent.AggroUnits`)
  (`AudioParameterControllerInterface.SetTriggerParameter` (`self.Goblin`) "Aggro"))

(fn `AttackSound`
  (`parent.AttackSound`)
  (`AudioParameterControllerInterface.SetTriggerParameter` (`self.Goblin`) "Attack"))

(fn `OnDeath`
  (`parent.OnDeath`)
  (`AudioParameterControllerInterface.SetTriggerParameter` (`self.Goblin`) "Death"))

(fn `OnHurt`
  (`parent.OnHurt`)
  (`AudioParameterControllerInterface.SetTriggerParameter` (`self.Goblin`) "TakeDamage"))

(fn `UserConstructionScript`
  (`parent.UserConstructionScript`))