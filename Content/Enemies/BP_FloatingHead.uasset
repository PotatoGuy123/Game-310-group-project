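; BP_FloatingHead is a floating head enemy that always faces the player and tracks whether it has a clear line of sight.
; Each tick it traces the Visibility channel to the player, ignoring the player, and sets CanAttack when nothing blocks the trace.
; It then snaps its full rotation toward the player.
; Death, hurt and attack sound functions only call the parent class.
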(event `self.ReceiveTick`
  (params (DeltaSeconds :type "Float (single-precision)"))
  (`self.CanSeePlayerCheck`)
  (`self.K2_SetActorRotation` (`KismetMathLibrary.FindLookAtRotation` (`self.K2_GetActorLocation`) (`self.K2_GetActorLocation` (`GameplayStatics.GetPlayerCharacter` 0)))))

(fn `AttackSound`
  (`parent.AttackSound`))

(fn `CanSeePlayerCheck`
  (bind (_outhit _returnvalue) (`KismetSystemLibrary.LineTraceSingle` (`self.K2_GetActorLocation`) (`self.K2_GetActorLocation` (`GameplayStatics.GetPlayerCharacter` 0)) "TraceTypeQuery1" false (`|MakeArray` (`GameplayStatics.GetPlayerCharacter` 0) :!type "Actor Object Reference")))
  (set `self.CanAttack` (not _returnvalue)))

(fn `OnDeath`
  (`parent.OnDeath`))

(fn `OnHurt`
  (`parent.OnHurt`))

(fn `UserConstructionScript`
  (`parent.UserConstructionScript`))