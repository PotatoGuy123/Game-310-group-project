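; Base enemy Blueprint that provides shared health, melee damage, death and slow behavior, with empty hook functions for hit, hurt, death, aggro and attack sound.
; Damage reaches HealthComponent a frame late, and its Die event spawns an actor, hides the enemy and destroys it after a delay.
; AttackCollider starts disabled and damages Player-tagged actors on overlap.
; Slow temporarily cuts walk speed, using chained timers for duration and cooldown.
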(event `self.ReceiveBeginPlay`
  (add `/Game/BluePrints/Component/HealthComponent.Die` (`self.HealthComponent`) (delegate `Die`))
  (`PrimitiveComponent.IgnoreActorWhenMoving` (`self.CapsuleComponent`) (`GameplayStatics.GetPlayerCharacter` 0) true)
  (`PrimitiveComponent.SetCollisionEnabled` (`self.AttackCollider`) "NoCollision")
  (set `self.DefaultMaxWalkSpeed` (`CharacterMovementComponent.MaxWalkSpeed` (`self.CharacterMovement`))))

(event `Die`
  (`self.OnDeath`)
  (`|SpawnActorFromClass` "/Game/BluePrints/BP_AlchoholPickup.BP_AlchoholPickup_C" (`self.GetTransform`) "Undefined" "MultiplyWithRoot" null null)
  (`self.SetActorEnableCollision` false)
  (`self.SetActorHiddenInGame` true)
  (`KismetSystemLibrary.Delay` 1.0)
  (`self.K2_DestroyActor`))

(event `/Game/BluePrints/Component/BPI_HealthInterface.TakeDamage`
  (params (DamageAmount :type "Float (double-precision)"))
  (`KismetSystemLibrary.DelayUntilNextFrame`)
  (`/Game/BluePrints/Component/HealthComponent.TakeDamage` (`self.HealthComponent`) DamageAmount)
  (`KismetSystemLibrary.PrintString` "I hurty")
  (`self.OnHurt`))

(event `self.AttackCollider.OnComponentBeginOverlap`
  (params (OverlappedComponent :type "PrimitiveComponent Object Reference") (OtherActor :type "Actor Object Reference") (OtherComp :type "PrimitiveComponent Object Reference") (OtherBodyIndex :type Integer) (bFromSweep :type Boolean) (SweepResult :type "HitResult Structure (by ref)"))
  (if (`self.ActorHasTag` OtherActor "Player")
    (message `/Game/BluePrints/Component/BPI_HealthInterface.TakeDamage` OtherActor (`self.Damage Amount`))
    (`self.Hit Effect` OtherActor)))

(event `/Game/BluePrints/Component/BPI_HealthInterface.HealDamage`
  (params (HealAmount :type "Float (double-precision)")))

(event `/Game/Enemies/AI/BPI_EnemyBase.Slow`
  (if (`self.CanBeSlowed`)
    (set `CharacterMovementComponent.MaxWalkSpeed` (/ (`self.DefaultMaxWalkSpeed`) 3.0) (`self.CharacterMovement`))
    (set `self.CanBeSlowed` false)
    (`KismetSystemLibrary.K2_SetTimerDelegate` (delegate `Stop Slow`) 3.0)))

(event `Stop Slow`
  (set `CharacterMovementComponent.MaxWalkSpeed` (`self.DefaultMaxWalkSpeed`) (`self.CharacterMovement`))
  (`KismetSystemLibrary.K2_SetTimerDelegate` (delegate `CanBeSlowedTrue`) 3.0))

(event `CanBeSlowedTrue`
  (set `self.CanBeSlowed` true))

(fn `AggroUnits`)

(fn `AttackSound`)

(fn `Hit Effect`
  (params (`Other Actor` :type "Actor Object Reference")))

(fn `OnDeath`)

(fn `OnHurt`)

(fn `UserConstructionScript`)